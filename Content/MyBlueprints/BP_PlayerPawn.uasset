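; BP_PlayerPawn is a player pawn that sets up Enhanced Input according to its Index variable.
; On BeginPlay it gets its PlayerController and adds IMC_Default when Index is 0, or IMC_SecondDefault otherwise, to that controller's input subsystem.
; IA_Move only prints the pawn's display name, with no movement logic yet.
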(event Input|EnhancedActionEvents|EnhancedInputActionIA_Move
  (params (ActionValue :type Vector%202D%20Structure) (ElapsedSeconds :type Float%20%28double-precision%29) (TriggeredSeconds :type Float%20%28double-precision%29) (InputAction :type Input%20Action%20Object%20Reference :default "/Game/ThirdPerson/Input/Actions/IA_Move.IA_Move"))
  (:Triggered
    (Development|PrintString (Utilities|GetDisplayName self))))

(event EventBeginPlay
  (bind _asplayer_controller (Utilities|Casting|CastToPlayerController (Pawn|GetController)))
  (if (== (Variables|Default|GetIndex) 0)
    (Input|AddMappingContext (PlayerController|LocalPlayerSubsystems|GetEnhancedInputLocalPlayerSubsystem _asplayer_controller) "/Game/ThirdPerson/Input/IMC_Default.IMC_Default" 0 "(bIgnoreAllPressedKeysUntilRelease=True,bForceImmediately=False)")
    (else
      (Input|AddMappingContext (PlayerController|LocalPlayerSubsystems|GetEnhancedInputLocalPlayerSubsystem _asplayer_controller) "/Game/ThirdPerson/Input/IMC_SecondDefault.IMC_SecondDefault" 0 "(bIgnoreAllPressedKeysUntilRelease=True,bForceImmediately=False)"))))

(event Collision|EventActorBeginOverlap
  (params (OtherActor :type Actor%20Object%20Reference)))

(event EventTick
  (params (DeltaSeconds :type Float%20%28single-precision%29)))

(fn ConstructionScript)